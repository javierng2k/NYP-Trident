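; BP_Weapons is a weapon actor that other code can move between an equipped and a removed pose on a supplied component.
; On BeginPlay it builds a two-sword mesh array but always shows the first, DarkRepulus, with physics off.
; Equip and Remove both detach the actor, reattach its root to the passed component keeping world transform, then snap the mesh to a hardcoded relative offset and rotation specific to each state.
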(event EventBeginPlay
  (bind _staticmeshcomponent (Variables|Debug|GetStaticMeshComponent))
  (bind _output_get (Variables|Default|SetWepansModelArray (Utilities|Array|MakeArray "/Game/Game/Weapons/FBX/DarkRepulus/SM_DarkRepulus.SM_DarkRepulus" "/Game/Game/Weapons/FBX/EluciDator/SM_EluciDator.SM_EluciDator")))
  (Components|StaticMesh|SetStaticMesh _staticmeshcomponent (Utilities|Array|Get(acopy) _output_get))
  (Physics|SetSimulatePhysics _staticmeshcomponent false))

(event Collision|EventActorBeginOverlap
  (params (OtherActor :type Actor%20Object%20Reference)))

(event EventTick
  (params (DeltaSeconds :type Float%20%28single-precision%29)))

(event EventEquip
  (params (AttachTo :type Scene%20Component%20Object%20Reference))
  (bind _staticmeshcomponent (Variables|Debug|GetStaticMeshComponent))
  (Physics|SetSimulatePhysics _staticmeshcomponent false)
  (Transformation|DetachFromActor "KeepWorld" "KeepWorld" "KeepWorld")
  (Transformation|AttachComponentToComponent (VehicleSound|GetRootComponent) AttachTo "None" "KeepWorld" "KeepWorld" "KeepWorld" false)
  (Transformation|SetRelativeLocationAndRotation _staticmeshcomponent "-2.000000,0.000000,0.000000" "-110.000000, 0,0.000000" false false))

(event EventRemove
  (params (AttachTo :type Scene%20Component%20Object%20Reference))
  (Physics|SetSimulatePhysics (Variables|Debug|GetStaticMeshComponent) false)
  (Transformation|DetachFromActor "KeepWorld" "KeepWorld" "KeepWorld")
  (Transformation|AttachComponentToComponent (VehicleSound|GetRootComponent) AttachTo "None" "KeepWorld" "KeepWorld" "KeepWorld" false)
  (Transformation|SetRelativeLocationAndRotation (Variables|Debug|GetStaticMeshComponent) "-20.000000,0.000000,30.000000" "90.000000,0.000000,90.000000" false false))

(fn ConstructionScript)