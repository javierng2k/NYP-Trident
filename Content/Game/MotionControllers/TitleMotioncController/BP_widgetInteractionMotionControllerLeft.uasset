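; Left-hand motion controller Blueprint that lets the player click UI widgets in the title area.
; The TriggerLeft input presses and releases a left mouse button pointer key on its WidgetInteraction component, turning the trigger into a widget click.
; A debug "left" string prints on each press, and the BeginPlay, overlap and Tick events are unused.
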(event EventBeginPlay
  (|CallParentFunction) ; This node is disabled and will not be called.\nDrag off pins to build functionality.
)

(event Collision|EventActorBeginOverlap
  (params (OtherActor :type Actor%20Object%20Reference)))

(event EventTick
  (params (DeltaSeconds :type Float%20%28single-precision%29))
  (|CallParentFunction DeltaSeconds) ; This node is disabled and will not be called.\nDrag off pins to build functionality.
)

(event Input|ActionEvents|InputActionTriggerLeft
  (params (Key :type Key%20Structure :default "None"))
  (:Pressed
    (Class|WidgetInteractionComponent|PressPointerKey (Variables|Default|GetWidgetInteraction) "LeftMouseButton")
    (Development|PrintString "left"))
  (:Released
    (Class|WidgetInteractionComponent|ReleasePointerKey (Variables|Default|GetWidgetInteraction) "LeftMouseButton")))

(fn ConstructionScript
  (|CallParentFunction))